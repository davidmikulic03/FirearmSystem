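; Test actor that reacts to bullet impact events with visual effects.
; OnPenetrate attaches a bullet hole decal aligned to the surface normal and spawns an NS_Impact Niagara burst; OnDestroy forwards to the same logic.
; OnRicochet spawns only a smaller burst, setting the particle count before activating the system, while OnHit does nothing.
; The decal fade-out is disconnected, so no timed fade is applied.
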(event EventBeginPlay)

(event Collision|EventActorBeginOverlap
  (params (OtherActor :type Actor%20Object%20Reference)))

(event EventTick
  (params (DeltaSeconds :type Float%20%28single-precision%29)))

(event EventOnHit
  (params (Bullet :type Bullet%20Object%20Reference) (Hit :type Hit%20Result%20Structure)))

(event EventOnPenetrate
  (params (Bullet :type Bullet%20Object%20Reference) (Location :type Vector :default "0, 0, 0") (Normal :type Vector :default "0, 0, 0"))
  (bind _returnvalue (Math|Conversions|RotationFromXVector Normal))
  (bind _returnvalue_2 (Class|GameplayStatics|SpawnDecalAttached "/Game/Art/Firearms/BulletHole/M_BulletHole.M_BulletHole" "5.000000,5.000000,5.000000" (Variables|Default|GetDefaultSceneRoot) "None" Location _returnvalue "KeepWorldPosition" 0.0))
  (Rendering|Components|Decal|SetFadeScreenSize _returnvalue_2 0.0)
  (bind _returnvalue_3 (Niagara|SpawnSystematLocation "/Game/Art/Firearms/NS_Impact.NS_Impact" Location _returnvalue "1.000000,1.000000,1.000000" true false))
  (Effects|Components|ParticleSystem|SetIntParameter _returnvalue_3 "Particles" 5)
  (Components|Activation|Activate _returnvalue_3 false))

(event EventOnRicochet
  (params (Bullet :type Bullet%20Object%20Reference) (Location :type Vector :default "0, 0, 0") (Normal :type Vector :default "0, 0, 0"))
  (bind _returnvalue (Niagara|SpawnSystematLocation "/Game/Art/Firearms/NS_Impact.NS_Impact" Location (Math|Conversions|RotationFromXVector Normal) "1.000000,1.000000,1.000000" true false))
  (Effects|Components|ParticleSystem|SetIntParameter _returnvalue "Particles" 3)
  (Components|Activation|Activate _returnvalue false))

(event EventOnDestroy
  (params (Bullet :type Bullet%20Object%20Reference) (Location :type Vector :default "0, 0, 0") (Normal :type Vector :default "0, 0, 0"))
  (Class|HittableActor|OnPenetrate Bullet Location Normal))

(fn ConstructionScript)